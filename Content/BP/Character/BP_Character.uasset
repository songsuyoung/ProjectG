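; BP_Character is a character Blueprint with an inventory component and debug output for items.
; The UseItem event only prints the received item ID and count to the screen.
; Pressing the 0 key fetches the inventory log from InventoryComponent and prints each entry.
; BeginPlay, Tick, overlap and the construction script contain no logic.
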(event `self.ReceiveActorBeginOverlap`
  (params (OtherActor :type "Actor Object Reference")))

(event `self.BP_UseItem`
  (params (ItemName :type Name) (Count :type Integer))
  (`KismetSystemLibrary.PrintString` (`KismetStringLibrary.Concat_StrStr` (`KismetStringLibrary.Concat_StrStr` "ItemID: " (`KismetStringLibrary.Conv_NameToString` ItemName)) (`KismetStringLibrary.Concat_StrStr` " ItemCount: " (`KismetStringLibrary.Conv_IntToString` Count)))))

(event `Key|Zero`
  (params (Key :type "Key Structure"))
  (:`Pressed`
    (bind _returnvalue (`GInventoryComponent.GetInventoryLog` (`self.InventoryComponent`)))
    (for _array_element _returnvalue
      (`KismetSystemLibrary.PrintString` _array_element))))

(fn `UserConstructionScript`)